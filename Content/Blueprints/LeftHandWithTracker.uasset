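; Left VR hand driven by a data glove, with a Vive tracker for wrist position and rock-paper-scissors gesture detection.
; Each tick copies the glove's rotations onto the wrist and finger bones in world space.
; With an HMD enabled, the glove's tracker offset places the hand mesh; otherwise the tracker is hidden.
; Glove gesture events set triggered and released flags for scissor, rock and paper, and ResetPose realigns glove orientation.
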(event `ResetPose`
  (`GloveComponent.OrientationAlignment` (`self.Glove`)))

(event `self.ReceiveTick`
  (params (DeltaSeconds :type "Float (single-precision)"))
  (`|ExecutionSequence`
    (:`then_0`
      (`self.UpdateHandPose`))
    (:`then_1`
      (if (`HeadMountedDisplayFunctionLibrary.IsHeadMountedDisplayEnabled`)
        (`self.UpdateWristPosition`)
        (else
          (`SceneComponent.SetVisibility` (`self.Vive_Tracker_0`) false false))))))

(event `self.Glove.Gesture_Triggered_0`
  (set `self.IsScissorTriggered` true))

(event `self.Glove.Gesture_Released_0`
  (set `self.IsScissorReleased` true))

(event `self.Glove.Gesture_Triggered_1`
  (set `self.IsRockTriggered` true))

(event `self.Glove.Gesture_Released_1`
  (set `self.IsRockReleased` true))

(event `self.Glove.Gesture_Triggered_2`
  (set `self.IsPaperTriggered` true))

(event `self.Glove.Gesture_Released_2`
  (set `self.IsPaperReleased` true))

(fn `UpdateHandPose`
  (bind _handmesh (`self.HandMesh`))
  (bind _rotation (`GloveComponent.rotation` (`self.Glove`)))
  (`PoseableMeshComponent.SetBoneRotationByName` _handmesh "wrist_l" (`|GetArrayItem` _rotation) "WorldSpace")
  (`PoseableMeshComponent.SetBoneRotationByName` _handmesh "finger_thumb_0_l" (`|GetArrayItem` _rotation 1) "WorldSpace")
  (`PoseableMeshComponent.SetBoneRotationByName` _handmesh "finger_thumb_1_l" (`|GetArrayItem` _rotation 2) "WorldSpace")
  (`PoseableMeshComponent.SetBoneRotationByName` _handmesh "finger_thumb_2_l" (`|GetArrayItem` _rotation 3) "WorldSpace")
  (`PoseableMeshComponent.SetBoneRotationByName` _handmesh "finger_index_0_l" (`|GetArrayItem` _rotation 4) "WorldSpace")
  (`PoseableMeshComponent.SetBoneRotationByName` _handmesh "finger_index_1_l" (`|GetArrayItem` _rotation 5) "WorldSpace")
  (`PoseableMeshComponent.SetBoneRotationByName` _handmesh "finger_index_2_l" (`|GetArrayItem` _rotation 6) "WorldSpace")
  (`PoseableMeshComponent.SetBoneRotationByName` _handmesh "finger_middle_0_l" (`|GetArrayItem` _rotation 7) "WorldSpace")
  (`PoseableMeshComponent.SetBoneRotationByName` _handmesh "finger_middle_1_l" (`|GetArrayItem` _rotation 8) "WorldSpace")
  (`PoseableMeshComponent.SetBoneRotationByName` _handmesh "finger_middle_2_l" (`|GetArrayItem` _rotation 9) "WorldSpace")
  (`PoseableMeshComponent.SetBoneRotationByName` _handmesh "finger_ring_0_l" (`|GetArrayItem` _rotation 10) "WorldSpace")
  (`PoseableMeshComponent.SetBoneRotationByName` _handmesh "finger_ring_1_l" (`|GetArrayItem` _rotation 11) "WorldSpace")
  (`PoseableMeshComponent.SetBoneRotationByName` _handmesh "finger_ring_2_l" (`|GetArrayItem` _rotation 12) "WorldSpace")
  (`PoseableMeshComponent.SetBoneRotationByName` _handmesh "finger_pinky_0_l" (`|GetArrayItem` _rotation 13) "WorldSpace")
  (`PoseableMeshComponent.SetBoneRotationByName` _handmesh "finger_pinky_1_l" (`|GetArrayItem` _rotation 14) "WorldSpace")
  (`PoseableMeshComponent.SetBoneRotationByName` _handmesh "finger_pinky_2_l" (`|GetArrayItem` _rotation 15) "WorldSpace"))

(fn `UpdateWristPosition`
  (bind _returnvalue (`GloveComponent.ApplyTrackerOffset` (`self.Glove`)))
  (`SceneComponent.K2_SetRelativeTransform` (`self.HandMesh`) _returnvalue false false))

(fn `UserConstructionScript`)