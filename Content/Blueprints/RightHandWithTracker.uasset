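; Right-hand VR Blueprint that drives a poseable hand mesh from a data glove paired with a Vive tracker.
; BeginPlay offsets the finger metacarpal bones; ResetPose realigns glove orientation.
; Each tick updates wrist alignment, copies glove rotations onto wrist and finger bones in world space, and applies the tracker-offset transform when an HMD is enabled, otherwise hiding the tracker.
; Glove gesture events set rock, paper and scissor trigger/release flags.
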(event `self.ReceiveBeginPlay`
  ;[1 1 1] Meta Joint Tuning
  (`self.MetaJointTuning`))

(event `ResetPose`
  ;[1 1 1] Reset Pose to Initial Pose
  (`GloveComponent.OrientationAlignment` (`self.Glove`)))

(event `self.ReceiveTick`
  (params (DeltaSeconds :type "Float (single-precision)"))
  (bind _glove (`self.Glove`))
  ;[1 1 1] Event Tick (Pose update)
  (`|ExecutionSequence`
    (:`then_0`
      (`GloveComponent.SetWristAlignment` _glove (`SceneComponent.K2_GetComponentRotation` (`self.Alignment`))))
    (:`then_1`
      (if (`GloveComponent.bIsDataGloveConnected` _glove)
        (`self.UpdateHandPose`)))
    (:`then_2`
      (if (`HeadMountedDisplayFunctionLibrary.IsHeadMountedDisplayEnabled`)
        (`self.UpdateWristPosition`)
        (else
          (`SceneComponent.SetVisibility` (`self.Vive_Tracker_0`) false false))))))

(event `self.Glove.Gesture_Triggered_0`
  ;[1 1 1] Gesture Event Handler
  (set `self.IsScissorTriggered` true))

(event `self.Glove.Gesture_Released_0`
  ;[1 1 1] Gesture Event Handler
  (set `self.IsScissorReleased` true))

(event `self.Glove.Gesture_Triggered_1`
  ;[1 1 1] Gesture Event Handler
  (set `self.IsRockTriggered` true))

(event `self.Glove.Gesture_Released_1`
  ;[1 1 1] Gesture Event Handler
  (set `self.IsRockReleased` true))

(event `self.Glove.Gesture_Triggered_2`
  ;[1 1 1] Gesture Event Handler
  (set `self.IsPaperTriggered` true))

(event `self.Glove.Gesture_Released_2`
  ;[1 1 1] Gesture Event Handler
  (set `self.IsPaperReleased` true))

(fn `MetaJointTuning`
  (bind _handmesh (`self.HandMesh`))
  (bind _returnvalue (`PoseableMeshComponent.GetBoneRotationByName` _handmesh "finger_index_meta_r" "ComponentSpace"))
  (`PoseableMeshComponent.SetBoneRotationByName` _handmesh "finger_index_meta_r" (`KismetMathLibrary.ComposeRotators` (struct :`Pitch` 5.0) _returnvalue) "ComponentSpace")
  (bind _returnvalue_2 (`PoseableMeshComponent.GetBoneRotationByName` _handmesh "finger_middle_meta_r" "ComponentSpace"))
  (`PoseableMeshComponent.SetBoneRotationByName` _handmesh "finger_middle_meta_r" (`KismetMathLibrary.ComposeRotators` (struct :`Pitch` 2.5) _returnvalue_2) "ComponentSpace")
  (bind _returnvalue_3 (`PoseableMeshComponent.GetBoneRotationByName` _handmesh "finger_ring_meta_r" "ComponentSpace"))
  (`PoseableMeshComponent.SetBoneRotationByName` _handmesh "finger_ring_meta_r" (`KismetMathLibrary.ComposeRotators` (struct :`Pitch` 1.0) _returnvalue_3) "ComponentSpace")
  (bind _returnvalue_4 (`PoseableMeshComponent.GetBoneRotationByName` _handmesh "finger_pinky_meta_r" "ComponentSpace"))
  (`PoseableMeshComponent.SetBoneRotationByName` _handmesh "finger_pinky_meta_r" (`KismetMathLibrary.ComposeRotators` (struct :`Pitch` -5.0) _returnvalue_4) "ComponentSpace"))

(fn `UpdateHandPose`
  (bind _handmesh (`self.HandMesh`))
  (bind _rotation (`GloveComponent.rotation` (`self.Glove`)))
  (`PoseableMeshComponent.SetBoneRotationByName` _handmesh "wrist_r" (`|GetArrayItem` _rotation) "WorldSpace")
  (`PoseableMeshComponent.SetBoneRotationByName` _handmesh "finger_thumb_0_r" (`|GetArrayItem` _rotation 1) "WorldSpace")
  (`PoseableMeshComponent.SetBoneRotationByName` _handmesh "finger_thumb_1_r" (`|GetArrayItem` _rotation 2) "WorldSpace")
  (`PoseableMeshComponent.SetBoneRotationByName` _handmesh "finger_thumb_2_r" (`|GetArrayItem` _rotation 3) "WorldSpace")
  (`PoseableMeshComponent.SetBoneRotationByName` _handmesh "finger_index_0_r" (`|GetArrayItem` _rotation 4) "WorldSpace")
  (`PoseableMeshComponent.SetBoneRotationByName` _handmesh "finger_index_1_r" (`|GetArrayItem` _rotation 5) "WorldSpace")
  (`PoseableMeshComponent.SetBoneRotationByName` _handmesh "finger_index_2_r" (`|GetArrayItem` _rotation 6) "WorldSpace")
  (`PoseableMeshComponent.SetBoneRotationByName` _handmesh "finger_middle_0_r" (`|GetArrayItem` _rotation 7) "WorldSpace")
  (`PoseableMeshComponent.SetBoneRotationByName` _handmesh "finger_middle_1_r" (`|GetArrayItem` _rotation 8) "WorldSpace")
  (`PoseableMeshComponent.SetBoneRotationByName` _handmesh "finger_middle_2_r" (`|GetArrayItem` _rotation 9) "WorldSpace")
  (`PoseableMeshComponent.SetBoneRotationByName` _handmesh "finger_ring_0_r" (`|GetArrayItem` _rotation 10) "WorldSpace")
  (`PoseableMeshComponent.SetBoneRotationByName` _handmesh "finger_ring_1_r" (`|GetArrayItem` _rotation 11) "WorldSpace")
  (`PoseableMeshComponent.SetBoneRotationByName` _handmesh "finger_ring_2_r" (`|GetArrayItem` _rotation 12) "WorldSpace")
  (`PoseableMeshComponent.SetBoneRotationByName` _handmesh "finger_pinky_0_r" (`|GetArrayItem` _rotation 13) "WorldSpace")
  (`PoseableMeshComponent.SetBoneRotationByName` _handmesh "finger_pinky_1_r" (`|GetArrayItem` _rotation 14) "WorldSpace")
  (`PoseableMeshComponent.SetBoneRotationByName` _handmesh "finger_pinky_2_r" (`|GetArrayItem` _rotation 15) "WorldSpace"))

(fn `UpdateWristPosition`
  (bind _returnvalue (`GloveComponent.ApplyTrackerOffset` (`self.Glove`)))
  (`SceneComponent.K2_SetRelativeTransform` (`self.HandMesh`) _returnvalue false false))

(fn `UserConstructionScript`)