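; Displays three left-hand meshes posed as scissor, rock and paper gestures that light up when triggered.
; On BeginPlay it builds each pose procedurally by setting component-space rotations on every finger bone of its poseable mesh, with no animation assets.
; Triggered and released events for each gesture print a debug message and swap that hand's material between a highlight color and the default.
; Nothing in this Blueprint detects gestures or calls those events.
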(event `self.ReceiveBeginPlay`
  (bind _paper (`self.Paper`))
  (bind _scissor (`self.Scissor`))
  (bind _rock (`self.Rock`))
  (`PoseableMeshComponent.SetBoneRotationByName` _scissor "finger_index_0_l" (struct :`Pitch` 10.0 :`Yaw` 90.0 :`Roll` 180.0) "ComponentSpace")
  (`PoseableMeshComponent.SetBoneRotationByName` _scissor "finger_index_1_l" (struct :`Pitch` 10.0 :`Yaw` 90.0 :`Roll` 180.0) "ComponentSpace")
  (`PoseableMeshComponent.SetBoneRotationByName` _scissor "finger_index_2_l" (struct :`Pitch` 10.0 :`Yaw` 90.0 :`Roll` 180.0) "ComponentSpace")
  (`PoseableMeshComponent.SetBoneRotationByName` _scissor "finger_middle_0_l" (struct :`Pitch` -5.0 :`Yaw` 90.0 :`Roll` 180.0) "ComponentSpace")
  (`PoseableMeshComponent.SetBoneRotationByName` _scissor "finger_middle_1_l" (struct :`Pitch` -5.0 :`Yaw` 90.0 :`Roll` 180.0) "ComponentSpace")
  (`PoseableMeshComponent.SetBoneRotationByName` _scissor "finger_middle_2_l" (struct :`Pitch` -5.0 :`Yaw` 90.0 :`Roll` 180.0) "ComponentSpace")
  (`PoseableMeshComponent.SetBoneRotationByName` _scissor "finger_ring_0_l" (struct :`Yaw` 170.0 :`Roll` 180.0) "ComponentSpace")
  (`PoseableMeshComponent.SetBoneRotationByName` _scissor "finger_ring_1_l" (struct :`Yaw` 250.0 :`Roll` 180.0) "ComponentSpace")
  (`PoseableMeshComponent.SetBoneRotationByName` _scissor "finger_ring_2_l" (struct :`Yaw` 340.0 :`Roll` 180.0) "ComponentSpace")
  (`PoseableMeshComponent.SetBoneRotationByName` _scissor "finger_pinky_0_l" (struct :`Yaw` 170.0 :`Roll` 180.0) "ComponentSpace")
  (`PoseableMeshComponent.SetBoneRotationByName` _scissor "finger_pinky_1_l" (struct :`Yaw` 250.0 :`Roll` 180.0) "ComponentSpace")
  (`PoseableMeshComponent.SetBoneRotationByName` _scissor "finger_pinky_2_l" (struct :`Yaw` 340.0 :`Roll` 180.0) "ComponentSpace")
  (`PoseableMeshComponent.SetBoneRotationByName` _scissor "finger_thumb_0_l" (struct :`Pitch` 20.0 :`Yaw` 130.0 :`Roll` -90.0) "ComponentSpace")
  (`PoseableMeshComponent.SetBoneRotationByName` _scissor "finger_thumb_1_l" (struct :`Pitch` -20.0 :`Yaw` 130.0 :`Roll` -90.0) "ComponentSpace")
  (`PoseableMeshComponent.SetBoneRotationByName` _scissor "finger_thumb_2_l" (struct :`Pitch` -60.0 :`Yaw` 130.0 :`Roll` -90.0) "ComponentSpace")
  (`PoseableMeshComponent.SetBoneRotationByName` _rock "finger_index_0_l" (struct :`Yaw` 170.0 :`Roll` 180.0) "ComponentSpace")
  (`PoseableMeshComponent.SetBoneRotationByName` _rock "finger_index_1_l" (struct :`Yaw` 250.0 :`Roll` 180.0) "ComponentSpace")
  (`PoseableMeshComponent.SetBoneRotationByName` _rock "finger_index_2_l" (struct :`Yaw` 340.0 :`Roll` 180.0) "ComponentSpace")
  (`PoseableMeshComponent.SetBoneRotationByName` _rock "finger_middle_0_l" (struct :`Yaw` 170.0 :`Roll` 180.0) "ComponentSpace")
  (`PoseableMeshComponent.SetBoneRotationByName` _rock "finger_middle_1_l" (struct :`Yaw` 250.0 :`Roll` 180.0) "ComponentSpace")
  (`PoseableMeshComponent.SetBoneRotationByName` _rock "finger_middle_2_l" (struct :`Yaw` 340.0 :`Roll` 180.0) "ComponentSpace")
  (`PoseableMeshComponent.SetBoneRotationByName` _rock "finger_ring_0_l" (struct :`Yaw` 170.0 :`Roll` 180.0) "ComponentSpace")
  (`PoseableMeshComponent.SetBoneRotationByName` _rock "finger_ring_1_l" (struct :`Yaw` 250.0 :`Roll` 180.0) "ComponentSpace")
  (`PoseableMeshComponent.SetBoneRotationByName` _rock "finger_ring_2_l" (struct :`Yaw` 340.0 :`Roll` 180.0) "ComponentSpace")
  (`PoseableMeshComponent.SetBoneRotationByName` _rock "finger_pinky_0_l" (struct :`Yaw` 170.0 :`Roll` 180.0) "ComponentSpace")
  (`PoseableMeshComponent.SetBoneRotationByName` _rock "finger_pinky_1_l" (struct :`Yaw` 250.0 :`Roll` 180.0) "ComponentSpace")
  (`PoseableMeshComponent.SetBoneRotationByName` _rock "finger_pinky_2_l" (struct :`Yaw` 340.0 :`Roll` 180.0) "ComponentSpace")
  (`PoseableMeshComponent.SetBoneRotationByName` _rock "finger_thumb_0_l" (struct :`Pitch` 20.0 :`Yaw` 130.0 :`Roll` -90.0) "ComponentSpace")
  (`PoseableMeshComponent.SetBoneRotationByName` _rock "finger_thumb_1_l" (struct :`Pitch` -20.0 :`Yaw` 130.0 :`Roll` -90.0) "ComponentSpace")
  (`PoseableMeshComponent.SetBoneRotationByName` _rock "finger_thumb_2_l" (struct :`Pitch` -60.0 :`Yaw` 130.0 :`Roll` -90.0) "ComponentSpace")
  (`PoseableMeshComponent.SetBoneRotationByName` _paper "finger_index_0_l" (struct :`Pitch` 10.0 :`Yaw` 90.0 :`Roll` 180.0) "ComponentSpace")
  (`PoseableMeshComponent.SetBoneRotationByName` _paper "finger_index_1_l" (struct :`Pitch` 10.0 :`Yaw` 90.0 :`Roll` 180.0) "ComponentSpace")
  (`PoseableMeshComponent.SetBoneRotationByName` _paper "finger_index_2_l" (struct :`Pitch` 10.0 :`Yaw` 90.0 :`Roll` 180.0) "ComponentSpace")
  (`PoseableMeshComponent.SetBoneRotationByName` _paper "finger_middle_0_l" (struct :`Pitch` 5.0 :`Yaw` 90.0 :`Roll` 180.0) "ComponentSpace")
  (`PoseableMeshComponent.SetBoneRotationByName` _paper "finger_middle_1_l" (struct :`Pitch` 5.0 :`Yaw` 90.0 :`Roll` 180.0) "ComponentSpace")
  (`PoseableMeshComponent.SetBoneRotationByName` _paper "finger_middle_2_l" (struct :`Pitch` 5.0 :`Yaw` 90.0 :`Roll` 180.0) "ComponentSpace")
  (`PoseableMeshComponent.SetBoneRotationByName` _paper "finger_ring_0_l" (struct :`Pitch` -5.0 :`Yaw` 90.0 :`Roll` 180.0) "ComponentSpace")
  (`PoseableMeshComponent.SetBoneRotationByName` _paper "finger_ring_1_l" (struct :`Pitch` -5.0 :`Yaw` 90.0 :`Roll` 180.0) "ComponentSpace")
  (`PoseableMeshComponent.SetBoneRotationByName` _paper "finger_ring_2_l" (struct :`Pitch` -5.0 :`Yaw` 90.0 :`Roll` 180.0) "ComponentSpace")
  (`PoseableMeshComponent.SetBoneRotationByName` _paper "finger_pinky_0_l" (struct :`Pitch` -10.0 :`Yaw` 90.0 :`Roll` 180.0) "ComponentSpace")
  (`PoseableMeshComponent.SetBoneRotationByName` _paper "finger_pinky_1_l" (struct :`Pitch` -10.0 :`Yaw` 90.0 :`Roll` 180.0) "ComponentSpace")
  (`PoseableMeshComponent.SetBoneRotationByName` _paper "finger_pinky_2_l" (struct :`Pitch` -10.0 :`Yaw` 90.0 :`Roll` 180.0) "ComponentSpace")
  (`PoseableMeshComponent.SetBoneRotationByName` _paper "finger_thumb_0_l" (struct :`Pitch` 20.0 :`Yaw` 120.0 :`Roll` -120.0) "ComponentSpace")
  (`PoseableMeshComponent.SetBoneRotationByName` _paper "finger_thumb_1_l" (struct :`Pitch` 20.0 :`Yaw` 120.0 :`Roll` -120.0) "ComponentSpace")
  (`PoseableMeshComponent.SetBoneRotationByName` _paper "finger_thumb_2_l" (struct :`Pitch` 20.0 :`Yaw` 120.0 :`Roll` -120.0) "ComponentSpace"))

(event `OnScissorTriggered`
  (`KismetSystemLibrary.PrintString` "scissor is triggered!")
  (`PrimitiveComponent.SetMaterial` (`self.Scissor`) 0 "/VRTRIXGlove/Materials/cyan.cyan"))

(event `OnScissorReleased`
  (`KismetSystemLibrary.PrintString` "scissor is released!")
  (`PrimitiveComponent.SetMaterial` (`self.Scissor`) 0 "/VRTRIXGlove/Materials/default.default"))

(event `OnRockTriggered`
  (`KismetSystemLibrary.PrintString` "rock is triggered!")
  (`PrimitiveComponent.SetMaterial` (`self.Rock`) 0 "/VRTRIXGlove/Materials/green.green"))

(event `OnRockReleased`
  (`KismetSystemLibrary.PrintString` "rock is  released!")
  (`PrimitiveComponent.SetMaterial` (`self.Rock`) 0 "/VRTRIXGlove/Materials/default.default"))

(event `OnPaperTriggered`
  (`KismetSystemLibrary.PrintString` "paper is triggered!")
  (`PrimitiveComponent.SetMaterial` (`self.Paper`) 0 "/VRTRIXGlove/Materials/yellow.yellow"))

(event `OnPaperReleased`
  (`KismetSystemLibrary.PrintString` "paper is  released!")
  (`PrimitiveComponent.SetMaterial` (`self.Paper`) 0 "/VRTRIXGlove/Materials/default.default"))

(fn `UserConstructionScript`)